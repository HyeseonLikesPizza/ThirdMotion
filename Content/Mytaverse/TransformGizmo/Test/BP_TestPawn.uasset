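; BP_TestPawn is a test pawn for selecting and transforming actors with BP_TransformGizmo using the mouse.
; Left-click feeds BPPointerInteractionComponent for hovered interactables, otherwise a visibility trace along the pointer ray selects an actor and activates the gizmo.
; Gizmo changes return through TransformEvent, which toggles the actor's root mobility while applying them.
; W/E/R/T switch gizmo modes, including combined translate-rotate, unless right mouse is held to allow movement.
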(event Custom|TransformEvent
  (params (Transform :type Transform))
  (bind _selectedactor (Variables|Default|GetSelectedActor)
    (:then
      (Transformation|SetMobility (Variables|/Script/Engine.Actor|GetRootComponent _selectedactor) "Movable")
      (Transformation|SetActorTransform _selectedactor Transform)
      (Transformation|SetMobility (Variables|/Script/Engine.Actor|GetRootComponent _selectedactor) "Static")
      (Transformation|SetMobility (Variables|/Script/Engine.Actor|GetRootComponent _selectedactor) "Movable"))
    (:else)))

(event EventBeginPlay
  (Variables|/Script/Engine.PlayerController|SetbShowMouseCursor (Game|GetPlayerController 0) true)
  (Default|SetupInteraction (Variables|Default|GetBP_PointerInteractionComponent) (Utilities|Struct|MakeFPointerInteractionSettings "NewEnumerator9" 1e+08 true 0.0 (Utilities|Array|MakeArray "ObjectTypeQuery2") true 0) true)
  (bind _returnvalue (Actor|GetActorOfClass "/Game/Mytaverse/TransformGizmo/BP_TransformGizmo.BP_TransformGizmo_C"))
  (bind _output_get (Variables|Default|SetGizmo _returnvalue))
  (Default|DeactivateGizmo _output_get) ; 一开始先不显示Gizmo
  (Input|SetIgnoreMoveInput (Game|GetPlayerController 0) true))

(event Input|MouseEvents|LeftMouseButton
  (params (Key :type Key%20Structure))
  (bind _returnvalue (Game|GetPlayerController 0))
  (bind _bp_pointerinteractioncomponent (Variables|Default|GetBP_PointerInteractionComponent))
  (bind _bp_pointerinteractioncomponent_2 (Variables|Default|GetBP_PointerInteractionComponent))
  (bind _outactor (Default|GetHoveredObject _bp_pointerinteractioncomponent_2))
  (bind (_raystart _rayend) (Default|GetPointerRay _bp_pointerinteractioncomponent_2))
  (:Pressed
    (Utilities|IsValid _outactor
      (:Is%20Valid
        (Default|PressPointer _bp_pointerinteractioncomponent)
        (Input|SetIgnoreLookInput _returnvalue true))))
  (:Released
    (Utilities|IsValid _outactor
      (:Is%20Valid
        (Default|ReleasePointer _bp_pointerinteractioncomponent)
        (Input|SetIgnoreLookInput _returnvalue false))
      (:Is%20Not%20Valid
        (bind _outhit (Collision|LineTraceByChannel _raystart _rayend "TraceTypeQuery1" true 0 "None"))
        (if (.bBlockingHit (Collision|BreakHitResult _outhit))
          (bind _output_get (Variables|Default|SetSelectedActor (.HitActor (Collision|BreakHitResult _outhit))))
          (Default|ActivateGizmo (Variables|Default|GetGizmo) (Transformation|GetActorTransform _output_get) (delegate Custom|TransformEvent)))))))

(event Input|KeyboardEvents|T
  (params (Key :type Key%20Structure))
  (:Pressed
    (if (not (Variables|Default|GetRightMousePressed))
      (Default|SetTransformMode (Variables|Default|GetGizmo) "NewEnumerator0" true))))

(event Input|KeyboardEvents|E
  (params (Key :type Key%20Structure))
  (:Pressed
    (if (not (Variables|Default|GetRightMousePressed))
      (Default|SetTransformMode (Variables|Default|GetGizmo) "NewEnumerator1" false))))

(event Input|MouseEvents|RightMouseButton
  (params (Key :type Key%20Structure))
  (bind _returnvalue (Game|GetPlayerController 0))
  (:Pressed
    (Variables|Default|SetRightMousePressed true)
    (Input|SetIgnoreMoveInput _returnvalue false))
  (:Released
    (Variables|Default|SetRightMousePressed false)
    (Input|SetIgnoreMoveInput _returnvalue true)))

(event Input|KeyboardEvents|W
  (params (Key :type Key%20Structure))
  (:Pressed
    (if (not (Variables|Default|GetRightMousePressed))
      (Default|SetTransformMode (Variables|Default|GetGizmo) "NewEnumerator0" false))))

(event Input|KeyboardEvents|R
  (params (Key :type Key%20Structure))
  (:Pressed
    (if (not (Variables|Default|GetRightMousePressed))
      (Default|SetTransformMode (Variables|Default|GetGizmo) "NewEnumerator2" false))))

(fn ConstructionScript)