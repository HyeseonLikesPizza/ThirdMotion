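; Player pawn for in-world editing that selects actors tagged "Edit" by mouse click and moves them with a shared transform gizmo.
; A cursor trace either starts a gizmo drag through the pointer interaction component, locking look input, or retargets the gizmo, with highlight toggling when switching actors.
; Gizmo changes apply locally and go to the server through ThirdMotionPlayerController, keyed by EditSyncComponent GUID.
; Escape clears the selection.
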(event Custom|TransformEvent
  (params (Transform :type Transform))
  ;[0.15 0.15 0.15 0.5] 선택한 액터가 Edit 액터일 때 Gizmo 활성화 [처음]
  (Class|ThirdMotionPlayerController|ServerRequestApplyTransform (Variables|Default|GetPlayerController) (.guid (Variables|/Script/ThirdMotion.EditSyncComponent|GetR_Meta (Actor|GetComponentbyClass (Variables|Default|GetTargetActor) "/Script/ThirdMotion.EditSyncComponent"))) Transform)
  (Transformation|SetActorTransform (Variables|Default|GetTargetActor) Transform))

(event Custom|DestroyGizmo
  ;[0.15 0.15 0.15 0.5] Destroy Gizmo
  (bind _targetactor (Variables|Default|GetTargetActor)
    (:then
      (Utilities|IsValid (Actor|GetComponentbyClass _targetactor "/Script/ThirdMotion.HighlightComponent")
        (:Is%20Valid
          (Class|HighlightComponent|EnableHighlight (Actor|GetComponentbyClass _targetactor "/Script/ThirdMotion.HighlightComponent") false)
          (Variables|Default|SetTargetActor 0)
          (Default|DeactivateGizmo (Variables|Default|GetGizmo))
          (Variables|/Script/ThirdMotion.ThirdMotionPlayerController|SetbGizmoShowed (Variables|Default|GetPlayerController) false))))
    (:else)))

(event Input|EnhancedActionEvents|EnhancedInputActionIA_Click
  (params (ActionValue :type Boolean) (ElapsedSeconds :type Float%20%28double-precision%29) (TriggeredSeconds :type Float%20%28double-precision%29) (InputAction :type Input%20Action%20Object%20Reference :default "/Game/Blueprints/Input/IA_Click.IA_Click"))
  (bind _returnvalue (Game|GetPlayerController 0))
  (bind (_hitresult _returnvalue_2) (Game|Player|GetHitResultUnderCursorbyChannel _returnvalue "TraceTypeQuery1" true))
  (bind (_bblockinghit _binitialoverlap _time _distance _location _impactpoint _normal _impactnormal _physmat _hitactor _hitcomponent) (Collision|BreakHitResult _hitresult))
  (:Triggered
    (if (not (Variables|Default|GetGizmoInitialized))
      ;[0.15 0.15 0.15 0.5] Gizmo 초기화
      (Variables|Default|SetGizmoInitialized true)
      (Default|PressPointer (Variables|Default|GetBP_PointerInteractionComponent))
      (if (Variables|/Game/Mytaverse/CoreBlueprints/PointerInteraction/BP_PointerInteractionComponent.BP_PointerInteractionComponent_C|GetbIsDragging (Variables|Default|GetBP_PointerInteractionComponent))
        (Input|SetIgnoreLookInput (Game|GetPlayerController 0) true))))
  (:Started
    (if _returnvalue_2
      (Variables|Default|SetHit%20Actor _hitactor)
      (if (Utilities|Enum|Equal(Enum) (Collision|GetCollisionObjectType _hitcomponent) "ECC_GameTraceChannel1")
        ;[0.15 0.15 0.15 0.5] Gizmo 초기화
        (if (not (Variables|Default|GetGizmoInitialized))
          (Variables|Default|SetGizmoInitialized true)
          (Default|PressPointer (Variables|Default|GetBP_PointerInteractionComponent))
          (if (Variables|/Game/Mytaverse/CoreBlueprints/PointerInteraction/BP_PointerInteractionComponent.BP_PointerInteractionComponent_C|GetbIsDragging (Variables|Default|GetBP_PointerInteractionComponent))
            (Input|SetIgnoreLookInput (Game|GetPlayerController 0) true)))
        (else
          (Variables|Default|GetTargetActor
            (:then
              (if (not (== (Variables|Default|GetHit%20Actor) (Variables|Default|GetTargetActor)))
                ;[0.15 0.15 0.15 0.5] 이미 선택된 액터가 있지만 또다른 Edit 가능한 액터를 선택
                (if (Actor|ActorHasTag (Variables|Default|GetHit%20Actor) "Edit")
                  (bind _targetactor (Variables|Default|GetTargetActor)
                    (:then
                      (Class|HighlightComponent|EnableHighlight (Actor|GetComponentbyClass _targetactor "/Script/ThirdMotion.HighlightComponent") false)
                      (bind _hit_actor (Variables|Default|GetHit%20Actor)
                        (:then
                          (Class|HighlightComponent|EnableHighlight (Actor|GetComponentbyClass _hit_actor "/Script/ThirdMotion.HighlightComponent") true)
                          ;[0.15 0.15 0.15 0.5] 선택한 액터가 Edit 액터일 때 Gizmo 활성화 [처음]
                          (Variables|Default|SetTargetActor (Variables|Default|GetHit%20Actor) :!label _label)
                          (Default|ActivateGizmo (Variables|Default|GetGizmo) (Transformation|GetActorTransform (Variables|Default|GetTargetActor)) (delegate Custom|TransformEvent))
                          (Variables|/Script/ThirdMotion.ThirdMotionPlayerController|SetbGizmoShowed (Variables|Default|GetPlayerController) true))
                        (:else)))
                    (:else)))))
            (:else
              (bind _hit_actor_2 (Variables|Default|GetHit%20Actor)
                (:then
                  (if (Actor|ActorHasTag _hit_actor_2 "Edit")
                    (goto _label)
                    (else
                      (CallFunction|DestroyGizmo))))
                (:else))))))))
  (:Completed
    ;[0.15 0.15 0.15 0.5] Gizmo Release
    (Default|ReleasePointer (Variables|Default|GetBP_PointerInteractionComponent))
    (Input|SetIgnoreLookInput (Game|GetPlayerController 0) false)
    (Variables|Default|SetGizmoInitialized false)))

(event EventBeginPlay
  ;[0.15 0.15 0.15 0.5] BeginPlay
  (Default|SetupInteraction (Variables|Default|GetBP_PointerInteractionComponent) (Utilities|Struct|MakeFPointerInteractionSettings "NewEnumerator9" 1e+08 true 0.0 (Utilities|Array|MakeArray "ObjectTypeQuery7") false 0 0 0 true true) true)
  (bind _returnvalue (Actor|GetActorOfClass "/Game/Mytaverse/TransformGizmo/BP_TransformGizmo.BP_TransformGizmo_C"))
  (Variables|Default|SetGizmo _returnvalue)
  (bind _asthird_motion_player_controller (Utilities|Casting|CastToThirdMotionPlayerController (Game|GetPlayerController 0)))
  (Variables|Default|SetPlayerController _asthird_motion_player_controller))

(event Input|KeyboardEvents|Escape
  (params (Key :type Key%20Structure :default "None"))
  ;[0.15 0.15 0.15 0.5] Destroy Gizmo
  (:Pressed
    (bind _targetactor (Variables|Default|GetTargetActor)
      (:then
        (Utilities|IsValid (Actor|GetComponentbyClass _targetactor "/Script/ThirdMotion.HighlightComponent")
          (:Is%20Valid
            (Class|HighlightComponent|EnableHighlight (Actor|GetComponentbyClass _targetactor "/Script/ThirdMotion.HighlightComponent") false)
            (Variables|Default|SetTargetActor 0)
            (Default|DeactivateGizmo (Variables|Default|GetGizmo))
            (Variables|/Script/ThirdMotion.ThirdMotionPlayerController|SetbGizmoShowed (Variables|Default|GetPlayerController) false))))
      (:else))))

(fn ConstructionScript)